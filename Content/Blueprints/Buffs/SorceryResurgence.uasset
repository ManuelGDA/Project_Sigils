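; Sorcery Resurgence buff component that enables spell recall on the player it is cast on for a limited time.
; On BeginPlay it sets the player's RecallSpells flag and copies SpellsToCast into SorceryResurgenceMemory, excluding its own spell, with debug prints.
; The duration scales with the player's SorceryResurgenceSpellCounter, after which it clears the flag and destroys itself.
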(event EventBeginPlay
  (bind _castedon (Variables|Default|GetCastedOn))
  (Utilities|FlowControl|Delay 0.05)
  (Utilities|IsValid _castedon
    (:Is%20Valid
      (bind _asbp_myplayer (Utilities|Casting|CastTobp_myplayer _castedon))
      (Variables|/Game/Blueprints/bp_myplayer.bp_myplayer_C|SetbRecallSpells? _asbp_myplayer true)
      (for _array_element (Variables|Default|GetSpellsToCast)
        (Development|PrintString (Utilities|String|Append _array_element " " (Utilities|String|ToString(Boolean) (Utilities|Enum|NotEqual(Enum) _array_element "SorceryResurgenceSpell"))) true true "(R=0.583333,G=0.437500,B=0.000000,A=1.000000)" 1e+01)
        (if (Utilities|Enum|NotEqual(Enum) _array_element "SorceryResurgenceSpell")
          (Utilities|Array|Add (Variables|/Game/Blueprints/bp_myplayer.bp_myplayer_C|GetSorceryResurgenceMemory _asbp_myplayer) _array_element)
          (else
            (Development|PrintString "Hello"))))
      (Utilities|FlowControl|Delay (* (Variables|/Game/Blueprints/bp_myplayer.bp_myplayer_C|GetSorceryResurgenceSpellCounter _asbp_myplayer) 2e+01))
      (Variables|/Game/Blueprints/bp_myplayer.bp_myplayer_C|SetbRecallSpells? _asbp_myplayer false)
      (Utilities|FlowControl|Delay 0.2)
      (Components|DestroyComponent))))