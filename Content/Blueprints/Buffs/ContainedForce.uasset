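; ContainedForce is a buff component that turns the next collision of its target, a player or projectile, into a radial force blast.
; Shortly after BeginPlay it binds to the hit event of the player's VR root or the projectile's mesh.
; On hit it fires the target's radial force, scaled by Magnitude, and spawns an element-specific emitter.
; It then unbinds, making it one-shot, and destroys itself after a delay.
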(event Custom|CE_UnleashContainedForce
  (params (HitComponent :type Primitive%20Component%20Object%20Reference) (OtherActor :type Actor%20Object%20Reference) (OtherComp :type Primitive%20Component%20Object%20Reference) (NormalImpulse :type Vector) (Hit :type Hit%20Result%20Structure%20%28by%20ref%29))
  (bind _magnitude (Variables|Default|GetMagnitude))
  (Variables|/Script/Engine.RadialForceComponent|SetImpulseStrength (Variables|/Game/Blueprints/bp_myplayer.bp_myplayer_C|GetRadialForceCenter (stale EventBeginPlay _asbp_myplayer)) (* _magnitude 3e+04))
  (Variables|/Script/Engine.RadialForceComponent|SetRadius (Variables|/Game/Blueprints/bp_myplayer.bp_myplayer_C|GetRadialForceCenter (stale EventBeginPlay _asbp_myplayer)) (* _magnitude 3e+02))
  (Effects|SpawnEmitteratLocation (Utilities|Select :Index (Variables|Default|GetElement) :NewEnumerator0 "/Game/AssetPacks/AdvancedMagicFX13/Particles/P_ky_flash2.P_ky_flash2" :NewEnumerator1 "/Game/AssetPacks/FXVarietyPack/Particles/P_ky_shotShockwave.P_ky_shotShockwave" :NewEnumerator2 "/Game/AssetPacks/FXVarietyPack/Particles/P_ky_waterBallHit.P_ky_waterBallHit" :NewEnumerator3 "/Game/AssetPacks/AdvancedMagicFX12/particles/P_ky_hit_thunder.P_ky_hit_thunder") (.location (Transformation|GetWorldTransform (Variables|/Game/Blueprints/bp_myplayer.bp_myplayer_C|GetRadialForceCenter (stale EventBeginPlay _asbp_myplayer)))) (.rotation (Transformation|GetWorldTransform (Variables|/Game/Blueprints/bp_myplayer.bp_myplayer_C|GetRadialForceCenter (stale EventBeginPlay _asbp_myplayer)))) (* "5.000000,5.000000,5.000000" (Variables|Default|GetMagnitude)))
  (Class|RadialForceComponent|FireImpulse (Variables|/Game/Blueprints/bp_myplayer.bp_myplayer_C|GetRadialForceCenter (stale EventBeginPlay _asbp_myplayer)))
  (Collision|UnbindEventfromOnComponentHit (.AsVRRoot%20Component (Utilities|Casting|CastToVRRootComponent (Variables|/Script/Engine.Actor|GetRootComponent (stale EventBeginPlay _asbp_myplayer)))) (delegate Custom|CE_UnleashContainedForce))
  (Utilities|FlowControl|Delay 5.0)
  (Components|DestroyComponent))

(event Custom|CE_UnleashContainedForceProjectile
  (params (HitComponent :type Primitive%20Component%20Object%20Reference) (OtherActor :type Actor%20Object%20Reference) (OtherComp :type Primitive%20Component%20Object%20Reference) (NormalImpulse :type Vector) (Hit :type Hit%20Result%20Structure%20%28by%20ref%29))
  (Effects|SpawnEmitteratLocation (Utilities|Select :Index (Variables|Default|GetElement) :NewEnumerator0 "/Game/AssetPacks/AdvancedMagicFX13/Particles/P_ky_flash2.P_ky_flash2" :NewEnumerator1 "/Game/AssetPacks/FXVarietyPack/Particles/P_ky_shotShockwave.P_ky_shotShockwave" :NewEnumerator2 "/Game/AssetPacks/FXVarietyPack/Particles/P_ky_waterBallHit.P_ky_waterBallHit" :NewEnumerator3 "/Game/AssetPacks/AdvancedMagicFX12/particles/P_ky_hit_thunder.P_ky_hit_thunder") (.location (Transformation|GetWorldTransform (Variables|/Game/Blueprints/bp_projectilefather.bp_projectilefather_C|GetStaticMesh (stale EventBeginPlay _asbp_projectilefather)))) (.rotation (Transformation|GetWorldTransform (Variables|/Game/Blueprints/bp_projectilefather.bp_projectilefather_C|GetStaticMesh (stale EventBeginPlay _asbp_projectilefather)))) (* "3.000000,3.000000,3.000000" (Variables|Default|GetMagnitude)))
  (Class|RadialForceComponent|FireImpulse (Variables|/Game/Blueprints/bp_projectilefather.bp_projectilefather_C|GetRadialForce (stale EventBeginPlay _asbp_projectilefather)))
  (Collision|UnbindEventfromOnComponentHit (Variables|/Game/Blueprints/bp_projectilefather.bp_projectilefather_C|GetStaticMesh (stale EventBeginPlay _asbp_projectilefather)) (delegate Custom|CE_UnleashContainedForceProjectile))
  (Utilities|FlowControl|Delay 5.0)
  (Components|DestroyComponent))

(event EventBeginPlay
  (bind _castedon (Variables|Default|GetCastedOn))
  (bind _magnitude (Variables|Default|GetMagnitude))
  (Utilities|FlowControl|Delay 0.05)
  (bind _asbp_myplayer (Utilities|Casting|CastTobp_myplayer _castedon)
    (:then
      (Collision|BindEventtoOnComponentHit (.AsVRRoot%20Component (Utilities|Casting|CastToVRRootComponent (Variables|/Script/Engine.Actor|GetRootComponent _asbp_myplayer))) (delegate Custom|CE_UnleashContainedForce)))
    (:CastFailed
      (bind _asbp_projectilefather (Utilities|Casting|CastTobp_projectilefather _castedon))
      (Variables|/Script/Engine.RadialForceComponent|SetImpulseStrength (Variables|/Game/Blueprints/bp_projectilefather.bp_projectilefather_C|GetRadialForce _asbp_projectilefather) (* _magnitude 3e+04))
      (Variables|/Script/Engine.RadialForceComponent|SetRadius (Variables|/Game/Blueprints/bp_projectilefather.bp_projectilefather_C|GetRadialForce _asbp_projectilefather) (* _magnitude 2.5e+02))
      (Collision|BindEventtoOnComponentHit (Variables|/Game/Blueprints/bp_projectilefather.bp_projectilefather_C|GetStaticMesh _asbp_projectilefather) (delegate Custom|CE_UnleashContainedForceProjectile)))))