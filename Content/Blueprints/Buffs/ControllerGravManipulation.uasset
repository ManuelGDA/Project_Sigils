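; Gravity-manipulation buff that puts whatever its cast target hits under magic control.
; Shortly after BeginPlay, if not self-cast, it binds to hit events on the target's static mesh root.
; On a hit, it disables gravity on the other actor's static or skeletal mesh root and passes it to GravManipulator.
; It unbinds after the first successful capture; nothing here restores gravity.
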(event Custom|SetupforGravManipulation
  (params (HitComponent :type Primitive%20Component%20Object%20Reference) (OtherActor :type Actor%20Object%20Reference) (OtherComp :type Primitive%20Component%20Object%20Reference) (NormalImpulse :type Vector) (Hit :type Hit%20Result%20Structure%20%28by%20ref%29))
  (bind _rootcomponent (Variables|/Script/Engine.Actor|GetRootComponent OtherActor))
  (Utilities|IsValid OtherActor
    (:Is%20Valid
      (bind _asstatic_mesh_component (Utilities|Casting|CastToStaticMeshComponent _rootcomponent)
        (:then
          (bind _output_get (Variables|Default|SetSMManipulated _asstatic_mesh_component))
          (Variables|Default|SetUseSMorSK true)
          (Physics|SetEnableGravity _output_get false)
          (Default|FAddforMagicControl (Variables|Default|GetGravManipulator) (Variables|Default|GetUseSMorSK) (Variables|Default|GetSMManipulated) (Variables|Default|GetSKManipulated) :!label _label)
          (Collision|UnbindEventfromOnComponentHit (stale EventBeginPlay _asstatic_mesh_component) (delegate Custom|SetupforGravManipulation))
          (Development|PrintString "timer set" true true "(R=0.234396,G=1.000000,B=0.121782,A=1.000000)" 5.0))
        (:CastFailed
          (bind _asskeletal_mesh_component (Utilities|Casting|CastToSkeletalMeshComponent _rootcomponent)
            (:then
              (bind _output_get_2 (Variables|Default|SetSKManipulated _asskeletal_mesh_component))
              (Variables|Default|SetUseSMorSK false)
              (Physics|SetEnableGravity _output_get_2 false)
              (goto _label))
            (:CastFailed
              (Development|PrintString "cast to sk failed" true true "(R=1.000000,G=0.036430,B=0.000000,A=1.000000)" 1e+01))))))))

(event EventBeginPlay
  (bind _castedon (Variables|Default|GetCastedOn))
  (Utilities|FlowControl|Delay 0.05)
  (if (not (Variables|Default|GetCastedOnSelf))
    (Utilities|IsValid _castedon
      (:Is%20Valid
        (bind _asstatic_mesh_component (Utilities|Casting|CastToStaticMeshComponent (Variables|/Script/Engine.Actor|GetRootComponent _castedon)))
        (Collision|BindEventtoOnComponentHit _asstatic_mesh_component (delegate Custom|SetupforGravManipulation))))))