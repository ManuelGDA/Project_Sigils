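; NoGrav is a timed buff component that switches off gravity on the actor it was cast on.
; After a brief delay on BeginPlay, it disables gravity on that actor's root, handling either a static mesh or a VR root component.
; When the duration ends, it restores gravity and destroys itself.
; An invalid target or other root type gets no effect, and the component is not destroyed.
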(event EventBeginPlay
  (bind _castedon (Variables|Default|GetCastedOn))
  (bind _duration (Variables|Default|GetDuration))
  (bind _rootcomponent (Variables|/Script/Engine.Actor|GetRootComponent _castedon))
  (Utilities|FlowControl|Delay 0.05)
  (Utilities|IsValid _castedon
    (:Is%20Valid
      (bind _asstatic_mesh_component (Utilities|Casting|CastToStaticMeshComponent _rootcomponent)
        (:then
          (Physics|SetEnableGravity _asstatic_mesh_component false)
          (Utilities|FlowControl|Delay _duration)
          (Physics|SetEnableGravity _asstatic_mesh_component true))
        (:CastFailed
          (bind _asvrroot_component (Utilities|Casting|CastToVRRootComponent _rootcomponent))
          (Physics|SetEnableGravity _asvrroot_component false)
          (Utilities|FlowControl|Delay _duration)
          (Physics|SetEnableGravity _asvrroot_component true)))
      (Components|DestroyComponent))))