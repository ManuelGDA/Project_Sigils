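; MusicManager is a Blueprint that plays a looping playlist of three background music cues through its Audio component.
; BeginPlay starts the first track by switching on SongCounter, which selects the cue to set and play.
; When the audio finishes, the counter increments and PlaySong runs again, resetting to zero and calling itself once past the last track.
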(event OnAudioFinished(Audio)
  (Math|Integer|IncrementInt (Variables|Default|GetSongCounter)
    (:%20%20
      (CallFunction|PlaySong))))

(event Custom|PlaySong
  (bind _audio (Variables|Default|GetAudio))
  (bind _audio_2 (Variables|Default|GetAudio))
  (bind _audio_3 (Variables|Default|GetAudio))
  (switch int (Variables|Default|GetSongCounter)
    (:0
      (Audio|Components|Audio|SetSound _audio_2 "/Game/AssetPacks/Desolace_OST/Cues/1_Lone_Explorer/3_Abandoned_Cue.3_Abandoned_Cue")
      (Audio|Components|Audio|Play _audio_2 0.0))
    (:1
      (Audio|Components|Audio|SetSound _audio_3 "/Game/AssetPacks/Desolace_OST/Cues/2_Island/2_Into_The_Deep_Cue.2_Into_The_Deep_Cue")
      (Audio|Components|Audio|Play _audio_3 0.0))
    (:2
      (Audio|Components|Audio|SetSound _audio "/Game/AssetPacks/Desolace_OST/Cues/5_Serenity_Peak/5_We_Made_It_Cue.5_We_Made_It_Cue")
      (Audio|Components|Audio|Play _audio 0.0))
    (:3
      (Variables|Default|SetSongCounter 0)
      (CallFunction|PlaySong))))

(event EventBeginPlay
  (bind _audio (Variables|Default|GetAudio))
  (bind _audio_2 (Variables|Default|GetAudio))
  (bind _audio_3 (Variables|Default|GetAudio))
  (switch int (Variables|Default|GetSongCounter)
    (:0
      (Audio|Components|Audio|SetSound _audio_2 "/Game/AssetPacks/Desolace_OST/Cues/1_Lone_Explorer/3_Abandoned_Cue.3_Abandoned_Cue")
      (Audio|Components|Audio|Play _audio_2 0.0))
    (:1
      (Audio|Components|Audio|SetSound _audio_3 "/Game/AssetPacks/Desolace_OST/Cues/2_Island/2_Into_The_Deep_Cue.2_Into_The_Deep_Cue")
      (Audio|Components|Audio|Play _audio_3 0.0))
    (:2
      (Audio|Components|Audio|SetSound _audio "/Game/AssetPacks/Desolace_OST/Cues/5_Serenity_Peak/5_We_Made_It_Cue.5_We_Made_It_Cue")
      (Audio|Components|Audio|Play _audio 0.0))
    (:3
      (Variables|Default|SetSongCounter 0)
      (CallFunction|PlaySong))))

(fn ConstructionScript)